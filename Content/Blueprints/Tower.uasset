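; Tower actor that automatically fires projectiles at enemies inside its Detector volume.
; Detector overlaps maintain the EnemiesDetected list, and the first detection starts a looping Attack timer that is never cleared.
; Each tick of that timer spawns a TowerProjectileBP at FirePoint, aimed at the first listed enemy if valid.
; CanAttack toggles around each shot but never gates firing, so the looping timer sets the rate.
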(event OnComponentEndOverlap(Detector)
  (params (OverlappedComponent :type Primitive%20Component%20Object%20Reference) (OtherActor :type Actor%20Object%20Reference) (OtherComp :type Primitive%20Component%20Object%20Reference) (OtherBodyIndex :type Integer))
  (bind _aspawn (Utilities|Casting|CastToPawn OtherActor))
  (bind _asenemy (Utilities|Casting|CastToEnemy _aspawn))
  (Utilities|Array|RemoveItem (Variables|Default|GetEnemiesDetected) _asenemy))

(event OnComponentBeginOverlap(Detector)
  (params (OverlappedComponent :type Primitive%20Component%20Object%20Reference) (OtherActor :type Actor%20Object%20Reference) (OtherComp :type Primitive%20Component%20Object%20Reference) (OtherBodyIndex :type Integer) (bFromSweep :type Boolean) (SweepResult :type Hit%20Result%20Structure%20%28by%20ref%29))
  (bind _aspawn (Utilities|Casting|CastToPawn OtherActor))
  (bind _asenemy (Utilities|Casting|CastToEnemy _aspawn))
  (Utilities|Array|Add (Variables|Default|GetEnemiesDetected) _asenemy)
  (if (not (Class|KismetSystemLibrary|IsTimerActive 0 "Attack"))
    (Utilities|Time|SetTimerbyFunctionName 0 "Attack" (Variables|Default|GetattackCooldown) true)))

(fn ConstructionScript)

(fn Attack
  (bind _enemiesdetected (Variables|Default|GetEnemiesDetected))
  (bind _output (Utilities|Array|Get(acopy) _enemiesdetected))
  ;[1 1 1] SpawnProjectole if sees enemy
  (if (!= (Utilities|Array|Length (Variables|Default|GetEnemiesDetected)) 0)
    (if true
      (if (Utilities|IsValid _output)
        (bind _returnvalue (Game|SpawnActorfromClass "/Game/Blueprints/TowerProjectileBP.TowerProjectileBP_C" (Transformation|GetWorldTransform (Variables|Default|GetFirePoint)) "Undefined" "MultiplyWithRoot" 0 0))
        (Default|InitProjectile _returnvalue _output)
        (Default|FireProjectile _returnvalue)
        (Variables|Default|SetcanAttack false)
        (Utilities|Time|SetTimerbyFunctionName 0 "Reset Attack" (Variables|Default|GetattackCooldown))))))

(fn ResetAttack
  (Variables|Default|SetcanAttack true))