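; The player's base in a wave-based defense game, holding HP and coins and handling win and loss.
; Hit, coin, spend and enemy-count events update the UI_PlayerStats HUD; spending assumes sufficient coins.
; Zero HP triggers PlayerLost, which shows the game-over widget, flags BP_SpawnManager as over and destroys all enemies.
; PlayerWon, not called here, shows the win widget and sets the same flag.
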(event Custom|GetCoins
  (params (Amount :type Integer))
  (bind _output_get (Variables|Default|SetCoins (+ Amount (Variables|Default|GetCoins))))
  (Default|ChangeCoins (Variables|Default|GetAs%20UI%20Player%20Stats) _output_get))

(event Custom|OnSpend
  (params (SpendCointAmount :type Integer))
  (bind _output_get (Variables|Default|SetCoins (- (Variables|Default|GetCoins) SpendCointAmount)))
  (Default|ChangeCoins (Variables|Default|GetAs%20UI%20Player%20Stats) _output_get))

(event Custom|UpdateEnemiesUI
  (params (Amount :type Integer))
  (Default|ChangeEnemy (Variables|Default|GetAs%20UI%20Player%20Stats) Amount))

(event Custom|SetupEnemyUI
  (params (Amount :type Integer))
  (bind _as_ui_player_stats (Variables|Default|GetAs%20UI%20Player%20Stats))
  (Default|ChangeEnemy _as_ui_player_stats Amount)
  (Default|SetWaveCount _as_ui_player_stats Amount))

(event EventBeginPlay
  (bind _health_widget (Variables|Default|GetHealth_Widget))
  (bind _returnvalue (UserInterface|GetWidget _health_widget))
  (bind _asui_player_stats (Utilities|Casting|CastToUI_PlayerStats _returnvalue))
  (Widget|GetAllWidgetsOfClass "/Game/UI/UI_PlayerStats.UI_PlayerStats_C" true)
  (UserInterface|Viewport|AddtoViewport _returnvalue 0)
  (bind _output_get (Variables|Default|SetAs%20UI%20Player%20Stats _asui_player_stats))
  (Default|ChangeHP _output_get (Math|Float|Truncate (Variables|Default|GetHP)))
  (Default|ChangeCoins _output_get (Variables|Default|GetCoins)))

(event EventGetHit
  (params (Damage :type Float%20%28double-precision%29))
  (Variables|Default|SetHP (- (Variables|Default|GetHP) Damage))
  (Audio|PlaySound2D "/Game/Audio/SFX/SFX_Base_Hit.SFX_Base_Hit" 1.0 1.0 0.0 0 0)
  (Default|ChangeHP (Variables|Default|GetAs%20UI%20Player%20Stats) (Math|Float|Truncate (Variables|Default|GetHP)))
  (if (<= (Variables|Default|GetHP) 0.0)
    (CallFunction|PlayerLost)))

(fn ConstructionScript)

(fn PlayerLost
  (Viewport|RemoveAllWidgets)
  (UserInterface|Viewport|AddtoViewport (UserInterface|GetWidget (Variables|Default|GetGG_Widget)) 0)
  (Variables|/Script/Engine.PlayerController|SetbShowMouseCursor (Game|GetPlayerController 0) true)
  (bind _outactors (Actor|GetAllActorsOfClass "/Game/Blueprints/BP_SpawnManager.BP_SpawnManager_C"))
  (Variables|/Game/Blueprints/BP_SpawnManager.BP_SpawnManager_C|SetIsGameOver (Utilities|Array|Get(acopy) _outactors) true)
  (bind _outactors_2 (Actor|GetAllActorsOfClass "/Game/Blueprints/Enemy.Enemy_C"))
  (for _array_element _outactors_2
    (Actor|DestroyActor _array_element)))

(fn PlayerWon
  (Viewport|RemoveAllWidgets)
  (UserInterface|Viewport|AddtoViewport (UserInterface|GetWidget (Variables|Default|GetWin_Widget)) 0)
  (Variables|/Script/Engine.PlayerController|SetbShowMouseCursor (Game|GetPlayerController 0) true)
  (bind _outactors (Actor|GetAllActorsOfClass "/Game/Blueprints/BP_SpawnManager.BP_SpawnManager_C"))
  (Variables|/Game/Blueprints/BP_SpawnManager.BP_SpawnManager_C|SetIsGameOver (Utilities|Array|Get(acopy) _outactors) true))