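; PlacementManager handles mouse-driven tower placement, paid for with the Base's coins.
; StartPlacement, called from the tower UI, checks affordability and spawns the real Tower actor as the ghost.
; While placing, Tick traces from the cursor and moves the ghost, slightly raised, over surfaces of a custom collision object type.
; MouseDown ends placement and charges the cost, without rechecking the surface under the cursor.
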(event Custom|StartPlacement
  ;[1 1 1] Called when pressed on tower building in ui
  (if (>= (Variables|/Game/Blueprints/Base.Base_C|GetCoins (Variables|Default|Getbase)) (Variables|Default|GetTowerCost))
    (Variables|Default|SetIsPlacing true)
    (bind _returnvalue (Game|SpawnActorfromClass "/Game/Blueprints/Tower.Tower_C" (Math|Transform|MakeTransform "0, 0, 0") "Undefined" "MultiplyWithRoot" 0 0))
    (Variables|Default|SetGhostRef _returnvalue)
    (else
      (Development|PrintString "need more"))))

(event Input|EnhancedActionEvents|EnhancedInputActionMouseDown
  (params (ActionValue :type Boolean) (ElapsedSeconds :type Float%20%28double-precision%29) (TriggeredSeconds :type Float%20%28double-precision%29) (InputAction :type Input%20Action%20Object%20Reference :default "/Game/InputSettings/MouseDown.MouseDown"))
  (if (Variables|Default|GetIsPlacing)
    (Variables|Default|SetIsPlacing false)
    (Default|OnSpend (Variables|Default|Getbase) (Variables|Default|GetTowerCost))))

(event EventTick
  (params (DeltaSeconds :type Float%20%28single-precision%29))
  (bind _returnvalue (Game|GetPlayerController 0))
  (bind (_worldlocation _worlddirection) (Game|Player|ConvertMouseLocationToWorldSpace _returnvalue))
  (if (Variables|Default|GetIsPlacing)
    (if (Utilities|IsValid (Variables|Default|GetGhostRef))
      (bind _outhit (Collision|LineTraceByChannel _worldlocation (+ _worldlocation (* _worlddirection (Math|Conversions|ToVector(Float) 1e+04))) "TraceTypeQuery1" false (Utilities|Array|MakeArray (Variables|Default|GetGhostRef)) "None"))
      (if (Utilities|Enum|Equal(Enum) (Collision|GetCollisionObjectType (.HitComponent (Collision|BreakHitResult _outhit))) "ECC_GameTraceChannel1")
        (Transformation|SetActorLocation (Variables|Default|GetGhostRef) (+ (.Location (Collision|BreakHitResult _outhit)) "0.000000,0.000000,40.000000") false false)
        (else
          (Development|PrintString (Utilities|String|ToString(Boolean) (Utilities|Enum|Equal(Enum) (Collision|GetCollisionObjectType (.HitComponent (Collision|BreakHitResult _outhit))) "ECC_GameTraceChannel1"))))))))

(event EventBeginPlay
  (bind _returnvalue (Game|GetPlayerController 0))
  ;[1 1 1] Comment
  (Variables|/Script/Engine.PlayerController|SetbShowMouseCursor _returnvalue true)
  (Input|AddMappingContext (PlayerController|LocalPlayerSubsystems|GetEnhancedInputLocalPlayerSubsystem _returnvalue) "/Game/InputSettings/NewInputMappingContext.NewInputMappingContext" 0 "(bIgnoreAllPressedKeysUntilRelease=True,bForceImmediately=False,bNotifyUserSettings=False)")
  (Input|EnableInput _returnvalue))

(fn ConstructionScript)