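; Enemy character for a wave-based base-defense game that walks a randomly chosen one of two BP_Path waypoint routes.
; An AIMoveTo loop advances through waypoints while it lives; overlapping the Base damages it and destroys the enemy.
; Hits update its health bar, and death awards coins, flags the death animation and leaves the spawn manager's list.
; Spawn unhides it, and a second-wave setup swaps the mesh and boosts speed and HP.
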(event Custom|Setup2ndWaveStats
  (Components|SkeletalMesh|SetSkeletalMeshAsset (Variables|Character|GetMesh) "/Game/EnemiesImport/BlackDrag/DragonSD_05.DragonSD_05")
  (Variables|Default|SetMove%20Speed (+ (Variables|Default|GetMove%20Speed) 75.0))
  (Variables|Default|SetHP (* (Variables|Default|GetHP) 2.0)))

(event EventBeginPlay
  (bind _final_path (Variables|Default|GetFinal%20Path))
  (bind _currentwaypointindex (Variables|Default|GetCurrentWaypointIndex))
  (bind _waypoints (Variables|/Game/Blueprints/BP_Path.BP_Path_C|GetWaypoints _final_path))
  (CallFunction|SetUpPathVariables)
  (CallFunction|SelectRandomPath)
  (Variables|/Script/Engine.CharacterMovementComponent|SetMaxWalkSpeed (Variables|Character|GetCharacterMovement) (Variables|Default|GetMove%20Speed))
  (Utilities|FlowControl|Delay 0.1)
  (AI|AIMoveTo self (Transformation|GetActorLocation (Utilities|Array|Get(acopy) _waypoints _currentwaypointindex)) 0 0.1 false :!label _label
    (:OnSuccess
      (Math|Integer|IncrementInt _currentwaypointindex
        (:%20%20
          (CallFunction|RotateEnemyTowardWaypoint)
          (if (< _currentwaypointindex (Utilities|Array|Length _waypoints))
            (Utilities|FlowControl|Delay 0.2)
            (if (> (Variables|Default|GetHP) 0.0)
              (goto _label))))))))

(event Collision|EventActorBeginOverlap
  (params (OtherActor :type Actor%20Object%20Reference))
  (bind _asbase (Utilities|Casting|CastToBase OtherActor))
  (Default|GetHit _asbase (Variables|Default|GetDamage))
  (Actor|DestroyActor))

(event EventGetHit
  (params (Damage :type Float%20%28double-precision%29))
  (Variables|Default|SetHP (- (Variables|Default|GetHP) Damage))
  (Audio|PlaySound2D "/Game/Audio/SFX/SFX_Arrow_hit.SFX_Arrow_hit" 1.0 1.0 0.0 0 0)
  (bind _ashealth_bar (Utilities|Casting|CastToHealthBar (UserInterface|GetUserWidgetObject (Variables|Default|GetEnemyHealthBar))))
  (Default|UpdateHealth _ashealth_bar (Variables|Default|GetHP) (Variables|Default|GetMaxHP))
  (if (<= (Variables|Default|GetHP) 0.0)
    (Default|GetCoins (Variables|Default|GetBase) (Variables|Default|GetCoinDrop))
    (bind _asred_drag_animation (Utilities|Casting|CastToRedDragAnimation (Components|SkeletalMesh|GetAnimInstance (Variables|Character|GetMesh))))
    (Variables|/Game/EnemiesImport/RedDragAnimation.RedDragAnimation_C|SetIsDead _asred_drag_animation true)
    (bind _returnvalue (Actor|GetActorOfClass "/Game/Blueprints/BP_SpawnManager.BP_SpawnManager_C"))
    (Utilities|Array|RemoveItem (Variables|/Game/Blueprints/BP_SpawnManager.BP_SpawnManager_C|GetEnemy%20Spawn%20List _returnvalue) self)))

(event EventSpawn
  (Rendering|SetActorHiddenInGame false))

(fn ConstructionScript)

(fn SetUpPathVariables
  (bind _outactors (Actor|GetAllActorsOfClass "/Game/Blueprints/BP_Path.BP_Path_C"))
  (Variables|Default|SetPath_1 (Utilities|Array|Get(acopy) _outactors))
  (Variables|Default|SetPath_2 (Utilities|Array|Get(acopy) _outactors 1)))

(fn SelectRandomPath
  (switch int (Math|Random|RandomInteger 2)
    (:Default
      (Variables|Default|SetFinal%20Path (Variables|Default|GetPath_2) :!label _label))
    (:0
      (Variables|Default|SetFinal%20Path (Variables|Default|GetPath_1)))
    (:1
      (goto _label))
    (:2
      (goto _label))))

(fn RotateEnemyTowardWaypoint
  (Transformation|SetActorRotation (Math|Rotator|MakeRotator (.Roll (Math|Rotator|BreakRotator (Math|Rotator|FindLookatRotation (Transformation|GetActorLocation) (Transformation|GetActorLocation (Utilities|Array|Get(acopy) (Variables|/Game/Blueprints/BP_Path.BP_Path_C|GetWaypoints (Variables|Default|GetFinal%20Path)) (Variables|Default|GetCurrentWaypointIndex)))))) 0.0 0.0)))