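; Spawn manager that runs two timed waves of AI enemies against a Base until the game is over.
; Tick accumulates a timer, spawns an Enemy at SpawnPoint each interval, links it to Base and updates the enemy count UI.
; Emptying wave one immediately starts wave two with boosted-or-altered stats via Setup2ndWaveStats.
; Once none remain to spawn and EnemySpawnList is empty, it tells Base the player won.
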(event EventBeginPlay
  (bind _output_get (Variables|Default|SetAmountLeft (Variables|Default|GetAmountToSpawnWave1)))
  (Utilities|FlowControl|Delay 0.2)
  (Default|SetupEnemyUI (Variables|Default|Getbase) _output_get))

(event EventTick
  (params (DeltaSeconds :type Float%20%28single-precision%29))
  (if (not (Variables|Default|GetIsGameOver))
    (bind _output_get (Variables|Default|SetSpawn%20Timer (+ DeltaSeconds (Variables|Default|GetSpawn%20Timer))))
    (if (>= _output_get (Variables|Default|GetSpawn%20Rate))
      (Variables|Default|SetSpawn%20Timer 0.0)
      (if (== (Variables|Default|GetAmountLeft) 0)
        ;[1 1 1] Not first time in second wave
        (if (== (Utilities|Array|Length (Variables|Default|GetEnemy%20Spawn%20List)) 0)
          (Default|PlayerWon (Variables|Default|Getbase)))
        (else
          (bind _returnvalue (AI|SpawnAIFromClass "/Game/Blueprints/Enemy.Enemy_C" 0 (Transformation|GetActorLocation (Variables|Default|GetSpawn%20Point)) "0, 0, 0" false 0))
          (bind _asenemy (Utilities|Casting|CastToEnemy _returnvalue))
          (Utilities|Array|Add (Variables|Default|GetEnemy%20Spawn%20List) _asenemy)
          (Variables|/Game/Blueprints/Enemy.Enemy_C|SetBase _asenemy (Variables|Default|Getbase))
          (if (Variables|Default|GetIs2ndWave)
            (Default|Setup2ndWaveStats _asenemy))
          (bind _output_get_2 (Variables|Default|SetAmountLeft (- (Variables|Default|GetAmountLeft) 1)))
          (Default|UpdateEnemiesUI (Variables|Default|Getbase) _output_get_2)
          (if (not (Variables|Default|GetIs2ndWave))
            ;[1 1 1] Set first time as second wave
            (bind _output_get_3 (Variables|Default|SetIs2ndWave (== _output_get_2 0)))
            ;[1 1 1] Enter 2nd wave first time
            (if _output_get_3
              (bind _output_get_4 (Variables|Default|SetAmountLeft (Variables|Default|GetAmountToSpawnWave2)))
              (Default|SetupEnemyUI (Variables|Default|Getbase) _output_get_4))))))))

(fn ConstructionScript)

(fn Spawn
  (params (Enemy :type Enemy%20Object%20Reference))
  (Rendering|SetActorHiddenInGame Enemy false)
  (Transformation|SetActorTransform Enemy (Transformation|GetActorTransform (Variables|Default|GetSpawn%20Point)))
  (Default|Spawn Enemy))