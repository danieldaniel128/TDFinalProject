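; Spawn manager that feeds timed waves of AI enemies at a spawn point and reports the remaining count to the Base's UI.
; Tick accumulates a timer, spawns an Enemy, passes it the Base and calls Setup2ndWaveStats on every spawn until game over.
; When the first count hits zero it refills once for a larger second wave; the trailing Delay gates nothing.
; A separate Spawn function repositions and unhides an existing enemy.
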(event EventBeginPlay
  (bind _output_get (Variables|Default|SetAmountLeft (Variables|Default|GetAmountToSpawn)))
  (Default|SetupEnemyUI (Variables|Default|Getbase) _output_get))

(event EventTick
  (params (DeltaSeconds :type Float%20%28single-precision%29))
  (if (not (or (> (Variables|Default|GetAmountLeft) (Variables|Default|GetAmountToSpawn)) (Variables|Default|GetIsGameOver)))
    (bind _output_get (Variables|Default|SetSpawn%20Timer (+ DeltaSeconds (Variables|Default|GetSpawn%20Timer))))
    (if (>= _output_get (Variables|Default|GetSpawn%20Rate))
      (Variables|Default|SetSpawn%20Timer 0.0)
      (bind _returnvalue (AI|SpawnAIFromClass "/Game/Yoav/Enemy.Enemy_C" 0 (Transformation|GetActorLocation (Variables|Default|GetSpawn%20Point)) "0, 0, 0" false 0))
      (bind _asenemy (Utilities|Casting|CastToEnemy _returnvalue))
      (Variables|/Game/Yoav/Enemy.Enemy_C|SetBase _asenemy (Variables|Default|Getbase))
      (Default|Setup2ndWaveStats _asenemy)
      (bind _output_get_2 (Variables|Default|SetAmountLeft (- (Variables|Default|GetAmountLeft) 1)))
      (Default|UpdateEnemiesUI (Variables|Default|Getbase) _output_get_2)
      (if (not (Variables|Default|GetIs2ndWave))
        (bind _output_get_3 (Variables|Default|SetIs2ndWave (== _output_get_2 0)))
        (if _output_get_3
          (bind _output_get_4 (Variables|Default|SetAmountToSpawn 50))
          (bind _output_get_5 (Variables|Default|SetAmountLeft _output_get_4))
          (Default|SetupEnemyUI (Variables|Default|Getbase) _output_get_5)
          (Utilities|FlowControl|Delay 5.0))))))

(fn ConstructionScript)

(fn Spawn
  (params (Enemy :type Enemy%20Object%20Reference))
  (Rendering|SetActorHiddenInGame Enemy false)
  (Transformation|SetActorTransform Enemy (Transformation|GetActorTransform (Variables|Default|GetSpawn%20Point)))
  (Default|Spawn Enemy))