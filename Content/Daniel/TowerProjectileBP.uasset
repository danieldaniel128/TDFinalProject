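; Arrow projectile for a tower that launches at an assigned enemy target and damages enemies it hits.
; On firing, it computes an arced launch velocity toward the target's current position without homing, plays a sound and self-destructs after a timeout.
; Each tick it rotates to face its velocity.
; Its hit sphere applies fixed damage to any overlapped Enemy through GetHit, then destroys the projectile after a short delay.
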(event OnComponentBeginOverlap(hitsphere)
  (params (OverlappedComponent :type Primitive%20Component%20Object%20Reference) (OtherActor :type Actor%20Object%20Reference) (OtherComp :type Primitive%20Component%20Object%20Reference) (OtherBodyIndex :type Integer) (bFromSweep :type Boolean) (SweepResult :type Hit%20Result%20Structure%20%28by%20ref%29))
  ;[1 1 1] hit enemy call hit event
  (bind _asenemy (Utilities|Casting|CastToEnemy OtherActor))
  (Default|GetHit _asenemy 1.75)
  (Utilities|FlowControl|Delay 0.2)
  (Actor|DestroyActor))

(event Custom|FireProjectile
  (bind _enemytarget (Variables|Default|GetEnemyTarget))
  (Utilities|IsValid _enemytarget
    (:Is%20Valid
      _)
    (:Is%20Not%20Valid
      _))
  (bind _outlaunchvelocity (Game|SuggestProjectileVelocityCustomArc (Transformation|GetActorLocation) (Transformation|GetActorLocation _enemytarget) 0.0 0.6))
  (Variables|/Script/Engine.MovementComponent|SetVelocity (Variables|Default|GetProjectileMovement) _outlaunchvelocity)
  (Audio|SpawnSound2D "/Game/Audio/SFX/SFX_Arrow_Fired.SFX_Arrow_Fired" 1.0 1.0 0.0 0)
  (Utilities|FlowControl|Delay 4.0)
  (Actor|DestroyActor))

(event Custom|InitProjectile
  (params (EnemyTarget :type Enemy%20Object%20Reference))
  (Variables|Default|SetEnemyTarget EnemyTarget))

(event EventTick
  (params (DeltaSeconds :type Float%20%28single-precision%29))
  (Transformation|SetActorRotation (Math|Rotator|MakeRotationfromAxes (Transformation|GetVelocity) "0, 0, 0" "0, 0, 0"))
  (if true
    _))

(fn ConstructionScript)